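; Robot control Blueprint that drives an industrial robot skeletal mesh through six motor values.
; Each tick it casts the mesh's anim instance to NewAnimBlueprint and copies the Motor1 to Motor6 variables into it.
; Pressing F plays a timeline that sets the mesh's relative yaw, rotating the whole robot.
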(event EventBeginPlay)

(event Collision|EventActorBeginOverlap
  (params (OtherActor :type Actor%20Object%20Reference)))

(event EventTick
  (params (DeltaSeconds :type Float%20%28single-precision%29))
  (bind _asnew_anim_blueprint (Utilities|Casting|CastToNewAnimBlueprint (Components|SkeletalMesh|GetAnimInstance (Variables|Default|GetSK_IndustrialRobot))))
  (Variables|/Game/Blueprints/NewAnimBlueprint.NewAnimBlueprint_C|Setmotor1 _asnew_anim_blueprint (Variables|Default|GetMotor1))
  (Variables|/Game/Blueprints/NewAnimBlueprint.NewAnimBlueprint_C|Setmotor2 _asnew_anim_blueprint (Variables|Default|GetMotor2))
  (Variables|/Game/Blueprints/NewAnimBlueprint.NewAnimBlueprint_C|Setmotor3 _asnew_anim_blueprint (Variables|Default|GetMotor3))
  (Variables|/Game/Blueprints/NewAnimBlueprint.NewAnimBlueprint_C|Setmotor4 _asnew_anim_blueprint (Variables|Default|GetMotor4))
  (Variables|/Game/Blueprints/NewAnimBlueprint.NewAnimBlueprint_C|Setmotor5 _asnew_anim_blueprint (Variables|Default|GetMotor5))
  (Variables|/Game/Blueprints/NewAnimBlueprint.NewAnimBlueprint_C|Setmotor6 _asnew_anim_blueprint (Variables|Default|GetMotor6)))

(event Input|KeyboardEvents|F
  (params (Key :type Key%20Structure :default "None"))
  (:Pressed
    (bind _newtrack_0 (Timeline|Rotate%20timeline Play)
      (:Update
        (Transformation|SetRelativeRotation (Variables|Default|GetSK_IndustrialRobot) (Math|Rotator|MakeRotator 0.0 0.0 _newtrack_0) false false)))))

(fn ConstructionScript)